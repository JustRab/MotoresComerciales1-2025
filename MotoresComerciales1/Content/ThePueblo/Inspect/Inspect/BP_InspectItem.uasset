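; Inspection actor that displays a given item's mesh for close-up viewing, with a widget showing its name and description.
; Inspect moves input from the character to this actor, and the interact action returns it, then removes the widget and destroys the actor.
; Mouse drag or move input rotates the mesh, while the wheel zooms via clamped SceneCapture2D FOV.
; Right-click resets rotation and zoom, and callers can set starting rotation and scale.
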(event `/Game/ThePueblo/Inspect/Inspect/InteractInterface.Inspect`
  (params (Character :type "/Game/ThePueblo/BaseBPs/BP_HorrorFirstPersonCharacter Object Reference") (InspectedItem :type "StaticMesh Object Reference") (ItemName :type Text) (ItemDescription :type Text))
  (bind _returnvalue (`GameplayStatics.GetPlayerControllerFromID` 0))
  ;[0.1417 0 0.15 0.5] Event Dispatcher
  (set `self.Character` Character)
  (`StaticMeshComponent.SetStaticMesh` (`self.Item`) InspectedItem)
  (bind _returnvalue_2 (`|CreateWidget` "/Game/ThePueblo/Inspect/Inspect/Widget/W_Inspect.W_Inspect_C" null ItemName ItemDescription))
  (bind _output_get (set `self.InspectWidgetReference` _returnvalue_2))
  (`UserWidget.AddToViewport` _output_get 0)
  (`self.DisableInput` (`self.Character`) _returnvalue)
  (`self.EnableInput` _returnvalue))

(event `EnhancedInput|/Game/ThirdPerson/Input/Actions/IA_Interact`
  (params (ActionValue :type Boolean) (ElapsedSeconds :type "Float (double-precision)") (TriggeredSeconds :type "Float (double-precision)") (InputAction :type "InputAction Object Reference" :default "/Game/ThirdPerson/Input/Actions/IA_Interact.IA_Interact"))
  (bind _returnvalue (`GameplayStatics.GetPlayerControllerFromID` 0))
  (bind _inspectwidgetreference (`self.InspectWidgetReference`))
  ;[0.15 0 0 0.5] Interact Action
  (:`Started`
    (`self.DisableInput` _returnvalue)
    (`self.EnableInput` (`self.Character`) _returnvalue)
    (`/Engine/EditorBlueprintResources/StandardMacros.IsValid` _inspectwidgetreference
      (:`Is Valid`
        (`Widget.RemoveFromParent` _inspectwidgetreference)
        (set `self.InspectWidgetReference` null)
        (`self.K2_DestroyActor`)))))

(event `Set Inspect Rotation`
  (params (`Item Rotation` :type "Rotator Structure"))
  (bind _item (`self.Item`))
  (bind (_returnvalue_location _returnvalue_rotation _returnvalue_scale) (`KismetMathLibrary.BreakTransform` (`SceneComponent.K2_GetComponentToWorld` _item)))
  ;[0.15 0.09692 0.03555 0.5] Set Inspection Rotation Dynamically
  (bind _output_get (set `self.Initial Rotation` `Item Rotation`))
  (`SceneComponent.K2_SetWorldTransform` _item (`KismetMathLibrary.MakeTransform` _returnvalue_location _output_get _returnvalue_scale) false false))

(event `Set Inspect Scale`
  (params (`Inspection Scale` :type "Vector Structure"))
  (bind _item (`self.Item`))
  (bind (_returnvalue_location _returnvalue_rotation) (`KismetMathLibrary.BreakTransform` (`SceneComponent.K2_GetComponentToWorld` _item)))
  ;[0.15 0.1387 0.06654 0.5] Set inspection Scale Dynamically
  (`SceneComponent.K2_SetWorldTransform` _item (`KismetMathLibrary.MakeTransform` _returnvalue_location _returnvalue_rotation `Inspection Scale`) false false))

(event `Key|LeftMouseButton`
  (params (Key :type "Key Structure"))
  ;[0.15 0.05201 0.02492 0.5] Rotate Allower
  (:`Pressed`
    (set `self.Rotate` true))
  (:`Released`
    (set `self.Rotate` false)))

(event `Key|RightMouseButton`
  (params (Key :type "Key Structure"))
  ;[0.15 0.0371 0 0.5] Resetting Transform of Inspect Item
  (:`Pressed`
    (`SceneComponent.K2_SetWorldRotation` (`self.Item`) (`self.Initial Rotation`) false false)
    (set `SceneCaptureComponent2D.FOVAngle` 50.0 (`self.SceneCaptureComponent2D`))))

(event `Key|MouseScrollUp`
  (params (Key :type "Key Structure"))
  (bind _scenecapturecomponent2d (`self.SceneCaptureComponent2D`))
  ;[0.15 0.0371 0 0.5] Zoom In
  (:`Pressed`
    (set `SceneCaptureComponent2D.FOVAngle` (`KismetMathLibrary.FClamp` (- (`SceneCaptureComponent2D.FOVAngle` _scenecapturecomponent2d) 1.0) 30.0 80.0) _scenecapturecomponent2d)))

(event `InputAxisKey|MouseX`
  (params (AxisValue :type "Float (single-precision)"))
  (bind _item (`self.Item`))
  ;[0.15 0.0371 0 0.5] Set Mouse Movement Horizontally
  (if (`self.Rotate`)
    (`SceneComponent.K2_SetWorldRotation` _item (`KismetMathLibrary.ComposeRotators` (`SceneComponent.K2_GetComponentRotation` _item) (`KismetMathLibrary.MakeRotator` 0.0 0.0 (* AxisValue -3.0))) false false)))

(event `Key|MouseScrollDown`
  (params (Key :type "Key Structure"))
  (bind _scenecapturecomponent2d (`self.SceneCaptureComponent2D`))
  ;[0.15 0.0371 0 0.5] Zoom Out
  (:`Pressed`
    (set `SceneCaptureComponent2D.FOVAngle` (`KismetMathLibrary.FClamp` (+ (`SceneCaptureComponent2D.FOVAngle` _scenecapturecomponent2d) 1.0) 30.0 80.0) _scenecapturecomponent2d)))

(event `InputAxisKey|MouseY`
  (params (AxisValue :type "Float (single-precision)"))
  (bind _item (`self.Item`))
  ;[0.15 0.0371 0 0.5] Set Mouse Movement Vertically
  (if (`self.Rotate`)
    (`SceneComponent.K2_SetWorldRotation` _item (`KismetMathLibrary.ComposeRotators` (`SceneComponent.K2_GetComponentRotation` _item) (`KismetMathLibrary.MakeRotator` 0.0 (* AxisValue -3.0))) false false)))

(event `EnhancedInput|/Game/ThirdPerson/Input/Actions/IA_Move`
  (params (ActionValue :type "Vector2D Structure") (ElapsedSeconds :type "Float (double-precision)") (TriggeredSeconds :type "Float (double-precision)") (InputAction :type "InputAction Object Reference" :default "/Game/ThirdPerson/Input/Actions/IA_Move.IA_Move"))
  (bind _item (`self.Item`))
  (bind _item_2 (`self.Item`))
  ;[0.15 0.0371 0 0.5] Move Item With WASD
  (:`Triggered`
    (if (or (!= ActionValue_X 0.0) (!= ActionValue_Y 0.0))
      (`|ExecutionSequence`
        (:`then_0`
          (`SceneComponent.K2_SetWorldRotation` _item_2 (`KismetMathLibrary.ComposeRotators` (`SceneComponent.K2_GetComponentRotation` _item_2) (`KismetMathLibrary.MakeRotator` 0.0 0.0 (* ActionValue_X -2.0))) false false))
        (:`then_1`
          (`SceneComponent.K2_SetWorldRotation` _item (`KismetMathLibrary.ComposeRotators` (`SceneComponent.K2_GetComponentRotation` _item) (`KismetMathLibrary.MakeRotator` 0.0 (* ActionValue_Y -2.0))) false false))))))

(fn `OnInteract`
  (params (Interactor :type "/Game/ThePueblo/BaseBPs/BP_HorrorFirstPersonCharacter Object Reference"))
  (return))

(fn `UserConstructionScript`)