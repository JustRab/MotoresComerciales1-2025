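; BP_BaseItem is a configurable base actor for world items that show interaction icons and can be inspected.
; Outer and inner spheres swap two icons as the player overlaps them, but the outer icon's hide-on-exit logic is disconnected.
; OnInteract, when Inspect is set, spawns a far-off BP_InspectItem and passes it the mesh, text, rotation and scale.
; The construction script applies mesh, scale, radii, icon location and debug sphere visibility.
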(event `self.outerSphereCollision.OnComponentBeginOverlap`
  (params (OverlappedComponent :type "PrimitiveComponent Object Reference") (OtherActor :type "Actor Object Reference") (OtherComp :type "PrimitiveComponent Object Reference") (OtherBodyIndex :type Integer) (bFromSweep :type Boolean) (SweepResult :type "HitResult Structure (by ref)"))
  (if (== OtherActor (`GameplayStatics.GetPlayerCharacter` 0))
    (`SceneComponent.SetVisibility` (`self.outerInteractionIcon`) true false)))

(event `self.outerSphereCollision.OnComponentEndOverlap`
  (params (OverlappedComponent :type "PrimitiveComponent Object Reference") (OtherActor :type "Actor Object Reference") (OtherComp :type "PrimitiveComponent Object Reference") (OtherBodyIndex :type Integer)))

(event `self.innerSphereCollision.OnComponentBeginOverlap`
  (params (OverlappedComponent :type "PrimitiveComponent Object Reference") (OtherActor :type "Actor Object Reference") (OtherComp :type "PrimitiveComponent Object Reference") (OtherBodyIndex :type Integer) (bFromSweep :type Boolean) (SweepResult :type "HitResult Structure (by ref)"))
  (if (== OtherActor (`GameplayStatics.GetPlayerCharacter` 0))
    (`SceneComponent.SetVisibility` (`self.outerInteractionIcon`) false false)
    (`SceneComponent.SetVisibility` (`self.innerInteractionIcon`) true false)))

(event `self.innerSphereCollision.OnComponentEndOverlap`
  (params (OverlappedComponent :type "PrimitiveComponent Object Reference") (OtherActor :type "Actor Object Reference") (OtherComp :type "PrimitiveComponent Object Reference") (OtherBodyIndex :type Integer))
  (if (== (`GameplayStatics.GetPlayerCharacter` 0) OtherActor)
    (`SceneComponent.SetVisibility` (`self.outerInteractionIcon`) true false)
    (`SceneComponent.SetVisibility` (`self.innerInteractionIcon`) false false)))

(event `self.ReceiveBeginPlay`
  (bind _asbp_horror_first_person_character (cast `/Game/ThePueblo/BaseBPs/BP_HorrorFirstPersonCharacter` (`GameplayStatics.GetPlayerCharacter` 0)))
  (set `self.BP Player Ref` _asbp_horror_first_person_character))

(event `/Game/ThePueblo/Inspect/Inspect/InteractInterface.OnInteract`
  (params (Interactor :type "/Game/ThePueblo/BaseBPs/BP_HorrorFirstPersonCharacter Object Reference"))
  (if (`self.Inspect?`)
    (bind _returnvalue (`|SpawnActorFromClass` "/Game/ThePueblo/Inspect/Inspect/BP_InspectItem.BP_InspectItem_C" (`KismetMathLibrary.MakeTransform` (100000000.0 0.0 0.0)) "Undefined" "MultiplyWithRoot" null null))
    (`/Game/ThePueblo/Inspect/Inspect/BP_InspectItem.Set Inspect Rotation` _returnvalue (`self.Item Inspection Rotation`))
    (`/Game/ThePueblo/Inspect/Inspect/BP_InspectItem.Set Inspect Scale` _returnvalue (`self.Item Inspection Scale`))
    (message `/Game/ThePueblo/Inspect/Inspect/InteractInterface.Inspect` _returnvalue Interactor (`StaticMeshComponent.StaticMesh` (`self.StaticMesh`)) (`self.ItemName`) (`self.ItemDescription`))))

(fn `UserConstructionScript`
  (bind _staticmesh (`self.StaticMesh`))
  (`|ExecutionSequence`
    (:`then_0`
      ;[0.05407 0.1305 0.15 0.5] Setting Sphere Radius
      (`SphereComponent.SetSphereRadius` (`self.innerSphereCollision`) (`self.innerSphereRadius`) true)
      (`SphereComponent.SetSphereRadius` (`self.outerSphereCollision`) (`self.outerSphereRadius`) true)
      ;[0.05007 0.1051 0.15 0.5] Setting Icon Locations
      (`SceneComponent.K2_SetRelativeLocation` (`self.innerInteractionIcon`) (`self.IconLocation`) false false)
      (`SceneComponent.K2_SetRelativeLocation` (`self.outerInteractionIcon`) (`self.IconLocation`) false false))
    (:`then_1`
      ;[0 0.009941 0.15 0.5] Setting Mesh Dinamically
      (`StaticMeshComponent.SetStaticMesh` (`self.StaticMesh`) (`self.ItemMesh`))
      ;[0 0.009941 0.15 0.5] Setting Mesh Transform Dynamically
      (`SceneComponent.K2_SetWorldTransform` _staticmesh (`KismetMathLibrary.MakeTransform` (`SceneComponent.K2_GetComponentLocation` _staticmesh) (`SceneComponent.K2_GetComponentRotation` _staticmesh) (`self.ItemScale`)) false false))
    (:`then_2`
      (if (`self.Debugging?`)
        (`SceneComponent.SetVisibility` (`self.innerSphereCollision`) true false)
        (`SceneComponent.SetVisibility` (`self.outerSphereCollision`) true false)
        (else
          (`SceneComponent.SetVisibility` (`self.innerSphereCollision`) false false)
          (`SceneComponent.SetVisibility` (`self.outerSphereCollision`) false false))))))