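; Actor Blueprint in the Visualizer folder that continuously spins and optionally bobs vertically, as an idle animation.
; BeginPlay caches the starting height, and Tick applies local yaw scaled by delta time while accumulating a time counter.
; When bob amplitude is positive, a remapped sine of that counter sets the height, oscillating between the starting Z and one amplitude below it.
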(event `self.ReceiveBeginPlay`
  (bind (_returnvalue_x _returnvalue_y _returnvalue_z) (`KismetMathLibrary.BreakVector` (`self.K2_GetActorLocation`)))
  ;[0 0.01341 0.15 0.5] Initialization
  (set `self.BaseZ` _returnvalue_z))

(event `self.ReceiveTick`
  (params (DeltaSeconds :type "Float (single-precision)"))
  ;[1 0.1818 0 0.5] Update (Rotation and Bobbing Effect)
  (`self.K2_AddActorLocalRotation` (`KismetMathLibrary.MakeRotator` 0.0 0.0 (* (`self.RotationSpeed`) DeltaSeconds)))
  (bind _output_get (set `self.TimeCounter` (+ DeltaSeconds (`self.TimeCounter`))))
  (if (> (`self.BobAmplitude`) 0.0)
    (set `self.OffsetZ` (/ (* (+ (`KismetMathLibrary.Sin` (* _output_get (`self.BobSpeed`))) 1.0) (* (`self.BobAmplitude`) -1.0)) 2.0))
    (bind _output_get_2 (set `self.NewZ` (+ (`self.BaseZ`) (`self.OffsetZ`))))
    (`self.K2_SetActorLocation` (`KismetMathLibrary.MakeVector` 0.0 0.0 _output_get_2))))

(fn `UserConstructionScript`)