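; Orbit camera that follows a target actor in the visualizer and rotates around it on player input.
; BeginPlay moves it to the target, resets the spring arm rotation and sets the arm length from Distance.
; Turn and LookUp axes add sensitivity-scaled local yaw and pitch to the arm, without clamping.
; Tick recenters on the target's colliding bounds, adjusted vertically by a fraction of their height and a fixed downward offset.
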(event `InputAxis|Turn`
  (params (AxisValue :type "Float (single-precision)"))
  ;[0.05596 0.651 0] Input Manager
  (`SceneComponent.K2_AddLocalRotation` (`self.SpringArm`) (`KismetMathLibrary.MakeRotator` 0.0 0.0 (* AxisValue (`self.Sensitivity_X`))) false false))

(event `self.ReceiveBeginPlay`
  (bind (_returnvalue_x _returnvalue_y _returnvalue_z) (`KismetMathLibrary.BreakVector` (`self.K2_GetActorLocation` (`self.TargetActor`))))
  ;[0 0.01421 0.15 0.5] Initialization
  (`/Engine/EditorBlueprintResources/StandardMacros.IsValid` (`self.TargetActor`)
    (:`Is Valid`
      (`self.K2_SetActorLocation` (`KismetMathLibrary.MakeVector` _returnvalue_x _returnvalue_y (- _returnvalue_z 25.0)))
      (`SceneComponent.K2_SetRelativeRotation` :`self` (`self.SpringArm`))
      (set `SpringArmComponent.TargetArmLength` (`self.Distance`) (`self.SpringArm`)))))

(event `InputAxis|LookUp`
  (params (AxisValue :type "Float (single-precision)"))
  ;[0.05596 0.651 0] Input Manager
  (`SceneComponent.K2_AddLocalRotation` (`self.SpringArm`) (`KismetMathLibrary.MakeRotator` 0.0 (* AxisValue (`self.Sensitivity_Y`))) false false))

(event `self.ReceiveTick`
  (params (DeltaSeconds :type "Float (single-precision)"))
  (bind _targetactor (`self.TargetActor`))
  (bind (_origin _boxextent) (`self.GetActorBounds` _targetactor true false))
  ;[1 0.193 0 0.5] Update
  (`/Engine/EditorBlueprintResources/StandardMacros.IsValid` _targetactor
    (:`Is Valid`
      (set `self.Center` _origin)
      (bind _output_get (set `self.ExtentZ` (.z _boxextent)))
      (bind (_returnvalue_x _returnvalue_y _returnvalue_z) (`KismetMathLibrary.BreakVector` (+ (`self.Center`) (`KismetMathLibrary.MakeVector` 0.0 0.0 (* _output_get 0.15)))))
      (`self.K2_SetActorLocation` (`KismetMathLibrary.MakeVector` _returnvalue_x _returnvalue_y (- _returnvalue_z 25.0))))))

(fn `UserConstructionScript`)