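; BP_Sumidero is a spawner actor that releases a batch of BP_DummyNPC actors around itself once, shortly after play begins.
; After a brief delay, BeginPlay calls SpawnbyTime, which loops from zero through ProjectileAmount inclusive, then prints a debug message.
; Each NPC spawns at a random reachable navmesh point within a fixed radius, with a yaw offset derived from the loop index and ProjectileAmount.
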(event `self.ReceiveBeginPlay`
  (`KismetSystemLibrary.Delay` 2.0)
  (`self.SpawnbyTime`))

(event `self.ReceiveTick`
  (params (DeltaSeconds :type "Float (single-precision)")))

(event `SpawnbyTime`
  (for _index (range (+ (- (`self.ProjectileAmount`) 0) 1))
    (`|SpawnActorFromClass` "/Game/Clases/BP_DummyNPC.BP_DummyNPC_C" (`KismetMathLibrary.MakeTransform` (`NavigationSystemV1.K2_GetRandomReachablePointInRadius` (`self.K2_GetActorLocation`) 500.0 null null) (`KismetMathLibrary.ComposeRotators` (`self.K2_GetActorRotation`) (`KismetMathLibrary.MakeRotator` 0.0 0.0 (`KismetMathLibrary.Conv_IntToDouble` (* _index (/ (`self.ProjectileAmount`) 300)))))) "Undefined" "MultiplyWithRoot" null null))
  (`KismetSystemLibrary.PrintText` "Acabo el loop"))

(fn `UserConstructionScript`)